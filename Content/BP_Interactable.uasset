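; Collectible actor that the player picks up with IA_Interact, lowering the Remaining count in Gamemode_FP.
; Its Collision component enables player 0's input on the actor only while a BP_Character overlaps it, while any actor overlap toggles the prompt Widget's visibility.
; Interacting decrements the counter, adds a new Collection_W widget to the viewport and destroys the actor.
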(event OnComponentBeginOverlap(Collision)
  (params (OverlappedComponent :type Primitive%20Component%20Object%20Reference) (OtherActor :type Actor%20Object%20Reference) (OtherComp :type Primitive%20Component%20Object%20Reference) (OtherBodyIndex :type Integer) (bFromSweep :type Boolean) (SweepResult :type Hit%20Result%20Structure%20%28by%20ref%29))
  (Utilities|Casting|CastToBP_Character OtherActor)
  (Input|EnableInput (Game|GetPlayerController 0)))

(event OnComponentEndOverlap(Collision)
  (params (OverlappedComponent :type Primitive%20Component%20Object%20Reference) (OtherActor :type Actor%20Object%20Reference) (OtherComp :type Primitive%20Component%20Object%20Reference) (OtherBodyIndex :type Integer))
  (Utilities|Casting|CastToBP_Character OtherActor)
  (Input|DisableInput (Game|GetPlayerController 0)))

(event Input|EnhancedActionEvents|EnhancedInputActionIA_Interact
  (params (ActionValue :type Boolean) (ElapsedSeconds :type Float%20%28double-precision%29) (TriggeredSeconds :type Float%20%28double-precision%29) (InputAction :type Input%20Action%20Object%20Reference :default "/Game/Inputs/IA_Interact.IA_Interact"))
  (:Started
    (bind _asgamemode_fp (Utilities|Casting|CastToGamemode_FP (Game|GetGameMode)))
    (bind _result (Math|Integer|DecrementInt (Variables|/Game/Gamemode_FP.Gamemode_FP_C|GetRemaining _asgamemode_fp))
      (:%20%20
        (Variables|/Game/Gamemode_FP.Gamemode_FP_C|SetRemaining _asgamemode_fp _result)
        (bind _returnvalue (UserInterface|CreateWidget "/Game/Widgets/Collection_W.Collection_W_C"))
        (UserInterface|Viewport|AddtoViewport _returnvalue 0)
        (Actor|DestroyActor)))))

(event Collision|EventActorBeginOverlap
  (params (OtherActor :type Actor%20Object%20Reference))
  (Rendering|SetVisibility (Variables|Default|GetWidget) true false))

(event Collision|EventActorEndOverlap
  (params (OtherActor :type Actor%20Object%20Reference))
  (Rendering|SetVisibility (Variables|Default|GetWidget) false false))

(fn ConstructionScript)